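; Goal actor for a plane game that rewards or punishes the player's arrival depending on score.
; CheckScore reads the score from PlaneGameMode and, once it passes a threshold, turns the mesh green and flags the mission as accomplished.
; When the player pawn overlaps it, an accomplished mission loads Minimal_Default as a level instance, while an unfinished one calls DestroyPlane on the Plane actor.
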(event `self.ReceiveActorBeginOverlap`
  (params (OtherActor :type "Actor Object Reference"))
  (if (== OtherActor (`GameplayStatics.GetPlayerPawn` 0))
    (if (`self.MissionAccomplished`)
      (`LevelStreamingDynamic.LoadLevelInstanceBySoftObjectPtr` "/Game/StarterContent/Maps/Minimal_Default.Minimal_Default" (0.0 0.0 0.0) (struct) "" null)
      (else
        (bind _returnvalue (`GameplayStatics.GetActorOfClass` "/Game/Blueprints/Plane.Plane_C"))
        (`/Game/Blueprints/Plane.DestroyPlane` _returnvalue)))))

(event `CheckScore`
  (bind _asplane_game_mode (cast `/Game/PlaneGameMode` (`GameplayStatics.GetGameMode`)))
  (if (> (`/Game/PlaneGameMode.Score` _asplane_game_mode) 5)
    (`PrimitiveComponent.SetMaterial` (`self.StaticMeshComponent`) 0 "/Engine/MapTemplates/Materials/Mat_DynamicGreen.Mat_DynamicGreen")
    (set `self.MissionAccomplished` true)))

(fn `UserConstructionScript`)